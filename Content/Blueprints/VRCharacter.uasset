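; Player character that moves in first-person style and draws on BP_WhiteBoard actors with the mouse, despite the VR name.
; EnableDraw toggles draw mode, which shows the cursor and blocks look input but not movement.
; While Draw or Erase is held, Tick traces from the cursor and sends the hit UV to the whiteboard's DrawOnWhiteboard.
; Erase behaves identically to Draw, and neither checks draw mode.
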(event `InputAction|EnableDraw`
  (params (Key :type "Key Structure"))
  (:`Pressed`
    (bind _output_get (set `self.IsCanDraw` (not (`self.IsCanDraw`))))
    (set `PlayerController.bShowMouseCursor` _output_get (`GameplayStatics.GetPlayerController` 0))))

(event `InputAxis|LookUp`
  (params (AxisValue :type "Float (single-precision)"))
  (if (not (`self.IsCanDraw`))
    (`self.AddControllerPitchInput` AxisValue)))

(event `InputAxis|Turn`
  (params (AxisValue :type "Float (single-precision)"))
  (if (not (`self.IsCanDraw`))
    (`self.AddControllerYawInput` AxisValue)))

(event `InputAxis|MoveForward`
  (params (AxisValue :type "Float (single-precision)"))
  (`self.AddMovementInput` (`KismetMathLibrary.GetForwardVector` (`KismetMathLibrary.MakeRotator` 0.0 0.0 (.yaw (`self.GetControlRotation`)))) AxisValue))

(event `InputAxis|MoveRight`
  (params (AxisValue :type "Float (single-precision)"))
  (`self.AddMovementInput` (`KismetMathLibrary.GetRightVector` (`KismetMathLibrary.MakeRotator` 0.0 0.0 (.yaw (`self.GetControlRotation`)))) AxisValue))

(event `InputAction|Draw`
  (params (Key :type "Key Structure"))
  (:`Pressed`
    (set `self.IsDrawing` true))
  (:`Released`
    (set `self.IsDrawing` false)))

(event `InputAction|Erase`
  (params (Key :type "Key Structure"))
  (:`Pressed`
    (set `self.IsDrawing` true))
  (:`Released`
    (set `self.IsDrawing` false)))

(event `self.ReceiveTick`
  (params (DeltaSeconds :type "Float (single-precision)"))
  (bind (_locationx _locationy) (`PlayerController.GetMousePosition` (`GameplayStatics.GetPlayerController` 0)))
  (bind (_worldposition _worlddirection) (`GameplayStatics.DeprojectScreenToWorld` (`GameplayStatics.GetPlayerController` 0) (`KismetMathLibrary.MakeVector2D` _locationx _locationy)))
  (`|ExecutionSequence`
    (:`then_0`
      (if (`self.IsDrawing`)
        (bind _outhit (`KismetSystemLibrary.LineTraceSingle` _worldposition (+ _worldposition (* _worlddirection 500.0)) "TraceTypeQuery1" true))
        (bind _asbp_white_board (cast `/Game/Blueprints/BP_WhiteBoard` (`.HitActor` (`GameplayStatics.BreakHitResult` _outhit))))
        (`/Game/Blueprints/BP_WhiteBoard.Draw On Whiteboard` _asbp_white_board (`GameplayStatics.FindCollisionUV` _outhit))))))

(fn `UserConstructionScript`)