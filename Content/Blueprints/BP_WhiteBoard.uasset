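; Whiteboard Blueprint that lets the player draw, erase and clear strokes on the RT_Whiteboard render target.
; DrawOnWhiteboard passes a 2D location to a dynamic marker or eraser material, chosen by the Erase hold input, and draws it into the target.
; The Graphic2D and Graphic3D inputs set the Version2D flag and save the target to disk as a PNG.
; The target clears to black on BeginPlay or Clear input.
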(event `InputAction|Erase`
  (params (Key :type "Key Structure"))
  (:`Pressed`
    (set `self.IsErasing` true))
  (:`Released`
    (set `self.IsErasing` false)))

(event `InputAction|Graphic2D`
  (params (Key :type "Key Structure"))
  (:`Pressed`
    (set `self.Version2D` true)
    (`self.SaveRenderTargetToDisk` "/Game/Materials/RT_Whiteboard.RT_Whiteboard" "RenderTarget.png")))

(event `InputAction|Graphic3D`
  (params (Key :type "Key Structure"))
  (:`Pressed`
    (set `self.Version2D` false)
    (`self.SaveRenderTargetToDisk` "/Game/Materials/RT_Whiteboard.RT_Whiteboard" "RenderTarget.png")))

(event `InputAction|Clear`
  (params (Key :type "Key Structure"))
  (:`Pressed`
    (`KismetRenderingLibrary.ClearRenderTarget2D` "/Game/Materials/RT_Whiteboard.RT_Whiteboard")))

(event `self.ReceiveBeginPlay`
  (`|ExecutionSequence`
    (:`then_0`
      (`self.EnableInput` (`GameplayStatics.GetPlayerController` 0)))
    (:`then_1`
      (bind _returnvalue (`KismetMaterialLibrary.CreateDynamicMaterialInstance` "/Game/Materials/M_WhiteBoardMarker.M_WhiteBoardMarker"))
      (set `self.WhiteboardMarker_MI` _returnvalue)
      (`KismetRenderingLibrary.ClearRenderTarget2D` "/Game/Materials/RT_Whiteboard.RT_Whiteboard"))
    (:`then_2`
      (bind _returnvalue_2 (`KismetMaterialLibrary.CreateDynamicMaterialInstance` "/Game/Materials/M_WhiteBoardMarkerErase.M_WhiteBoardMarkerErase"))
      (set `self.WhiteboardMarkerEraser_MI` _returnvalue_2))))

(event `Draw On Whiteboard`
  (params (LocationOnDraw :type "Vector2D Structure"))
  (bind _whiteboardmarker_mi (`self.WhiteboardMarker_MI`))
  (bind _whiteboardmarkereraser_mi (`self.WhiteboardMarkerEraser_MI`))
  (bind _returnvalue (`KismetMathLibrary.Conv_VectorToLinearColor` (`KismetMathLibrary.Conv_Vector2DToVector` LocationOnDraw)))
  (if (`self.IsErasing`)
    (`MaterialInstanceDynamic.SetVectorParameterValue` _whiteboardmarkereraser_mi "DrawLocation" _returnvalue)
    (`KismetRenderingLibrary.DrawMaterialToRenderTarget` "/Game/Materials/RT_Whiteboard.RT_Whiteboard" _whiteboardmarkereraser_mi)
    (else
      (`MaterialInstanceDynamic.SetVectorParameterValue` _whiteboardmarker_mi "DrawLocation" _returnvalue)
      (`KismetRenderingLibrary.DrawMaterialToRenderTarget` "/Game/Materials/RT_Whiteboard.RT_Whiteboard" _whiteboardmarker_mi))))

(fn `UserConstructionScript`)